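; BP_FireGuy is the playable fire avatar, which can hand player control to another pawn the camera points at.
; A one-time SoulSearch event adds its Enhanced Input mapping context, with only a debug print for a camera animation.
; Bird-named input actions drive look and actor-relative movement.
; The change-character action line-traces from the camera and possesses any pawn hit, leaving persistent debug lines and prints.
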(event `/Game/Avatars/BPI_ChangeChar.Soul Search`
  ;[1 1 1] Set Up Fire Inputs
  (`/Engine/EditorBlueprintResources/StandardMacros.DoOnce` false
    (:`Completed`
      (`KismetSystemLibrary.PrintString` "Play Camera Anim to actor")
      (bind _asplayer_controller (cast `PlayerController` (`self.GetController`)))
      (bind _returnvalue (pcsubsystem `EnhancedInputLocalPlayerSubsystem` _asplayer_controller))
      (`/Engine/EditorBlueprintResources/StandardMacros.IsValid` _returnvalue
        (:`Is Valid`
          (`EnhancedInputSubsystemInterface.AddMappingContext` _returnvalue null 0 (struct)))))))

(event `EnhancedInput|/Game/Avatars/Bird/IA_BirdCamera`
  (params (ActionValue :type "Vector2D Structure") (ElapsedSeconds :type "Float (double-precision)") (TriggeredSeconds :type "Float (double-precision)") (InputAction :type "InputAction Object Reference" :default "/Game/Avatars/Bird/IA_BirdCamera.IA_BirdCamera"))
  ;[1 1 1] Bird Look Round
  (:`Triggered`
    (`self.AddControllerYawInput` ActionValue_X)
    (`self.AddControllerPitchInput` (* ActionValue_Y -1.0))))

(event `self.ReceiveActorBeginOverlap`
  (params (OtherActor :type "Actor Object Reference")))

(event `EnhancedInput|/Game/Avatars/Bird/IA_MoveBird`
  (params (ActionValue :type "Vector2D Structure") (ElapsedSeconds :type "Float (double-precision)") (TriggeredSeconds :type "Float (double-precision)") (InputAction :type "InputAction Object Reference" :default "/Game/Avatars/Bird/IA_MoveBird.IA_MoveBird"))
  ;[1 1 1] Move
  (:`Triggered`
    (`self.AddMovementInput` (`self.GetActorRightVector`) ActionValue_X)
    (`self.AddMovementInput` (`self.GetActorForwardVector`) ActionValue_Y)))

(event `EnhancedInput|/Game/Avatars/IA_ChangeChar`
  (params (ActionValue :type Boolean) (ElapsedSeconds :type "Float (double-precision)") (TriggeredSeconds :type "Float (double-precision)") (InputAction :type "InputAction Object Reference" :default "/Game/Avatars/IA_ChangeChar.IA_ChangeChar"))
  (bind _camera (`self.Camera`))
  (bind _returnvalue (`SceneComponent.K2_GetComponentLocation` _camera))
  (:`Triggered`
    (bind _outhit (`KismetSystemLibrary.LineTraceSingle` _returnvalue (+ _returnvalue (* (`KismetMathLibrary.GetForwardVector` (`SceneComponent.K2_GetComponentRotation` _camera)) 10000.0)) "TraceTypeQuery2" false (`|MakeArray` self :!type "Actor Object Reference") "Persistent"))
    (`KismetSystemLibrary.PrintString` "working")
    (bind _aspawn (cast `Pawn` (`.HitActor` (`GameplayStatics.BreakHitResult` _outhit)))
      (:`then`
        (`Controller.Possess` (`GameplayStatics.GetPlayerController` 0) _aspawn))
      (:`CastFailed`
        (`KismetSystemLibrary.PrintString` "Cast failed")))))

(fn `UserConstructionScript`)